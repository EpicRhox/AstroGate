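; Game mode for a wave-based asteroid game, coordinating startup, score, pausing, wave restarts and saving.
; Once the HUD initializes, it runs a countdown and, after a matching fixed delay, has BP_Spawner spawn a wave or restore one cached in the game instance.
; Restart rolls score back to the wave-start value.
; SaveGame snapshots asteroids, score, wave and lives to a numbered slot; ship choice is still unsaved.
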(event `self.ReceiveBeginPlay`
  (bind _returnvalue (`GameplayStatics.GetPlayerController` 0))
  ;[0.15 0.1226 0.0162 0.5] Add game mode to input stack
  (`self.EnableInput` _returnvalue)
  ;[0.15 0.1105 0.005759 0.5] Save HUD blueprint reference
  (bind _asbp_hud (cast `/Game/Blueprints/BP_HUD` (`PlayerController.GetHUD` _returnvalue)))
  (set `self.HUD` _asbp_hud)
  ;[0.15 0.1137 0.008928 0.5] If spawner exists, save a reference. Otherwise warn us.
  (bind _returnvalue_2 (`GameplayStatics.GetActorOfClass` "/Game/Blueprints/BP_Spawner.BP_Spawner_C"))
  (`/Engine/EditorBlueprintResources/StandardMacros.IsValid` _returnvalue_2
    (:`Is Valid`
      (set `self.Spawner` _returnvalue_2)
      (add `/Game/Blueprints/BP_HUD.OnInitilized` (`self.HUD`) (delegate `HUDLoaded`)))
    (:`Is Not Valid`
      (`KismetSystemLibrary.PrintString` "NO SPAWNER ON MAP" true true (struct :`R` 0.686957 :`G` 0.001397 :`B` 1e-06 :`A` 1.0) 10.0))))

(event `HUDLoaded`
  (bind _asbp_my_game_instance (cast `/Game/Blueprints/BP_MyGameInstance` (`GameplayStatics.GetGameInstance`)))
  ;[0.15 0.1259 0.01707 0.5] Loading Save Game?
  (set `self.GameInstanceBP` _asbp_my_game_instance)
  (if (`/Game/Blueprints/BP_MyGameInstance.bIsLoadingFromSave` _asbp_my_game_instance)
    (set `/Game/Blueprints/BP_MyGameInstance.bIsLoadingFromSave` false _asbp_my_game_instance)
    (set `self.CurrentScore` (`/Game/Blueprints/BP_MyGameInstance.TempSavedScore` (`self.GameInstanceBP`)))
    (set `/Game/Blueprints/BP_Spawner.CurrentWave` (`/Game/Blueprints/BP_MyGameInstance.TempSavedWave` (`self.GameInstanceBP`)) (`self.Spawner`))
    (`self.GameStart`)
    (`KismetSystemLibrary.Delay` 3.1)
    (`/Game/Blueprints/BP_Spawner.LoadWaveFromSave` (`self.Spawner`) (`/Game/Blueprints/BP_MyGameInstance.TempSavedSpawned` (`self.GameInstanceBP`)))
    (else
      (`self.GameStart`)
      (`KismetSystemLibrary.Delay` 3.0)
      ;[0.15 0.09479 0.01049 0.5] Tell Spawner to spawn a wave
      (`/Game/Blueprints/BP_Spawner.SpawnWave` (`self.Spawner`)))))

(event `EnhancedInput|/Game/Input/IA_TogglePaused`
  (params (ActionValue :type Boolean) (ElapsedSeconds :type "Float (double-precision)") (TriggeredSeconds :type "Float (double-precision)") (InputAction :type "InputAction Object Reference" :default "/Game/Input/IA_TogglePaused.IA_TogglePaused"))
  (:`Started`
    (`self.PauseGame`)))

(event `PauseGame`
  ;[0.15 0.124 0.005361 0.5] Toggle Pause on/off
  (bind _output_get (set `self.IsPaused` (not (`self.IsPaused`))))
  (`GameplayStatics.SetGamePaused` _output_get)
  ;[0.15 0.1073 0.01013 0.5] Tell HUD to show/hide pause menu
  (`/Game/Blueprints/BP_HUD.SetPaused` (`self.HUD`) (`self.IsPaused`)))

(event `/Game/Blueprints/BPI_RestartGame.RestartGame`
  ;[0.15 0.1172 0.006776 0.5] Tell spawner to do its RestartGame
  (`/Game/Blueprints/BPI_RestartGame.RestartGame` (`self.Spawner`))
  ;[0.15 0.1166 0.01636 0.5] Tell player to reset its values
  (message `/Game/Blueprints/BPI_RestartGame.RestartGame` (`GameplayStatics.GetPlayerPawn` 0))
  ;[0.15 0.1169 0.0103 0.5] Reset Current Score to saved Wave Start Score
  (set `self.CurrentScore` (`self.WaveStartScore`))
  ;[0.15 0.1117 0.00478 0.5] Spawn new wave
  (`/Game/Blueprints/BP_Spawner.SpawnWave` (`self.Spawner`)))

(event `AddPoints`
  (params (Points :type Integer))
  ;[0.15 0.01942 0.01993 0.5] Add Score
  (set `self.CurrentScore` (+ Points (`self.CurrentScore`))))

(event `GameStart`
  (bind _hud (`self.HUD`))
  (bind _countdownwidget (`/Game/Blueprints/BP_HUD.CountdownWidget` _hud))
  (`WidgetBlueprintLibrary.SetInputMode_UIOnlyEx` (`GameplayStatics.GetPlayerController` 0) (`/Game/Blueprints/BP_HUD.CountdownWidget` (`self.HUD`)))
  ;[0.15 0.1233 0.006218 0.5] Save Score at the Beginning of Wave
  (`UserWidget.AddToViewport` (`/Game/Blueprints/BP_HUD.HUDWidget` _hud) 0)
  (add `/Game/Blueprints/BP_Spawner.NewWaveSpawned` (`self.Spawner`) (delegate `HandleWaveStartScore`))
  ;[0.15 0.033 0.01864 0.5] Start Countdown
  (`/Game/Art/WBP_Countdown.StartCountdown` _countdownwidget 3)
  (add `/Game/Art/WBP_Countdown.CountdownFinished` _countdownwidget (delegate `SpawnAfterCountdown`)))

(event `HandleWaveStartScore`
  ;[0.15 0.1233 0.006218 0.5] Save Score at the Beginning of Wave
  (set `self.WaveStartScore` (`self.CurrentScore`)))

(event `SpawnAfterCountdown`
  (`WidgetBlueprintLibrary.SetInputMode_GameOnly` (`GameplayStatics.GetPlayerController` 0)))

(fn `SaveGame`
  (params (SlotIndex :type Integer))
  (locals (EnemySnapshotArray :type "Array of /Game/Blueprints/F_EnemySaveData Structure"))
  (bind _outactors (`GameplayStatics.GetAllActorsOfClass` "/Game/Blueprints/BP_Asteroid.BP_Asteroid_C"))
  (for _array_element _outactors
    (bind _asbp_asteroid (cast `/Game/Blueprints/BP_Asteroid` _array_element))
    (`KismetArrayLibrary.Array_Add` (`local.EnemySnapshotArray`) (make `/Game/Blueprints/F_EnemySaveData` (`SceneComponent.K2_GetComponentToWorld` (`/Game/Blueprints/BP_Movement.DefaultSceneRoot` _asbp_asteroid)) (`MovementComponent.Velocity` (`/Game/Blueprints/BP_Movement.FloatingPawnMovement` _asbp_asteroid)) (`/Game/Blueprints/BP_Asteroid.Type` _asbp_asteroid))))
  (bind _returnvalue (`GameplayStatics.CreateSaveGameObject` "/Game/Blueprints/BP_GameSave.BP_GameSave_C"))
  (bind _output_get (set `self.GameSaveRef` _returnvalue))
  (set `/Game/Blueprints/BP_GameSave.SavedSpawned` (`local.EnemySnapshotArray`) _output_get)
  (set `/Game/Blueprints/BP_GameSave.SavedScore` (`self.CurrentScore`) (`self.GameSaveRef`))
  (set `/Game/Blueprints/BP_GameSave.SavedWave` (`/Game/Blueprints/BP_Spawner.CurrentWave` (`self.Spawner`)) (`self.GameSaveRef`))
  (bind _asbp_player (cast `/Game/Blueprints/BP_Player` (`GameplayStatics.GetPlayerPawn` 0)))
  (set `/Game/Blueprints/BP_GameSave.SavedLives` (`/Game/Blueprints/BP_Player.CurrentLives` _asbp_player) (`self.GameSaveRef`))
  (`GameplayStatics.SaveGameToSlot` (`self.GameSaveRef`) (`KismetStringLibrary.Concat_StrStr` "SaveSlot_" (`KismetStringLibrary.Conv_IntToString` SlotIndex))))

(fn `UserConstructionScript`)