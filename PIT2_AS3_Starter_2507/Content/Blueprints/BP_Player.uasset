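; Player ship pawn with thrust, rotation and held-fire shooting, using stats and mesh applied from ship data.
; Enhanced Input sets acceleration, yaw and a shooting flag; Tick spawns projectiles through a fire-rate Delay.
; BP_Killable deaths cost a life, then respawn the ship with temporary collision-off invulnerability and a timer-driven color blink.
; Lives initialize from the GameInstance save or default; running out shows Game Over and tells the GameMode to restart.
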(event `self.ReceiveBeginPlay`
  (`parent.ReceiveBeginPlay`)
  (bind _returnvalue (`KismetSystemLibrary.K2_SetTimerDelegate` (`|CreateDelegate` :!event `Blink`) 0.1 true))
  (bind _output_get (set `self.BlinkTimer` _returnvalue))
  (`KismetSystemLibrary.K2_PauseTimerHandle` _output_get)
  (bind _asbp_my_game_instance (cast `/Game/Blueprints/BP_MyGameInstance` (`GameplayStatics.GetGameInstance`)))
  (if (`/Game/Blueprints/BP_MyGameInstance.bIsLoadingFromSave` _asbp_my_game_instance)
    (`self.InitializePlayer` (`/Game/Blueprints/BP_MyGameInstance.TempSavedLives` _asbp_my_game_instance))
    (else
      (`self.InitializePlayer` 3)))
  (`self.RestartPlayer`)
  ;[1 1 1] When BP_Killable sends OnDeath event
  (add `/Game/Blueprints/BP_Killable.OnDeath` (`self.BP_Killable`) (delegate `OnDeath`)))

(event `OnDeath`
  ;[1 1 1] Disable movement
  (set `self.CanMove` false)
  ;[1 1 1] Remove a life and clamp
  (bind _output_get (set `self.CurrentLives` (`KismetMathLibrary.Clamp` (- (`self.CurrentLives`) 1) 0 3)))
  ;[1 1 1] Any lives left?
  (if (!= _output_get 0)
    ;[1 1 1] Yes. Respawn and make invulnerable for 3 seconds.
    (`self.RestartPlayer`)
    (bind _output_get_2 (set `self.IsInvulnerable` true))
    (`self.SetInvulnerable` _output_get_2)
    (`KismetSystemLibrary.K2_UnPauseTimerHandle` (`self.BlinkTimer`))
    (`KismetSystemLibrary.Delay` 3.0)
    (`KismetSystemLibrary.K2_PauseTimerHandle` (`self.BlinkTimer`))
    (`MeshComponent.SetVectorParameterValueOnMaterials` (`self.ShipMesh`) "Color" (1.0 1.0 1.0))
    (bind _output_get_3 (set `self.IsInvulnerable` false))
    (`self.SetInvulnerable` _output_get_3)
    (else
      ;[0.15 0.008968 0.01183 0.5] Show GameOver Screen upon death
      (bind _returnvalue (`GameplayStatics.GetActorOfClass` "/Game/Blueprints/BP_HUD.BP_HUD_C"))
      (bind _gameoverwidget (`/Game/Blueprints/BP_HUD.GameOverWidget` _returnvalue))
      (`UserWidget.AddToViewport` _gameoverwidget 0)
      (set `self.GameOverWidget` _gameoverwidget)
      (`KismetSystemLibrary.Delay` 3.0)
      (`Widget.RemoveFromParent` (`self.GameOverWidget`))
      ;[1 1 1] No. Tell game mode to restart game
      (message `/Game/Blueprints/BPI_RestartGame.RestartGame` (`GameplayStatics.GetGameMode`)))))

(event `self.ReceiveTick`
  (params (DeltaSeconds :type "Float (single-precision)"))
  ;[1 1 1] Movement
  (`parent.ReceiveTick` DeltaSeconds)
  ;[1 1 1] If shooting, can move, and is not invulnerable...
  (if (and (`self.IsShooting`) (`self.CanMove`) (not (`self.IsInvulnerable`)))
    ;[1 0.7748 0] Add Shoot Code Here
    (`KismetSystemLibrary.Delay` (`self.FireRate`))
    (`|SpawnActorFromClass` "/Game/Blueprints/BP_Projectile.BP_Projectile_C" (`KismetMathLibrary.MakeTransform` (`self.K2_GetActorLocation`) (`self.K2_GetActorRotation`) (0.25 0.25 0.25)) "Undefined" "MultiplyWithRoot" null null)))

(event `/Game/Blueprints/BPI_RestartGame.RestartGame`
  ;[1 1 1] Reset lives/score
  (`self.InitializePlayer` 3)
  ;[1 1 1] Stop and move the ship.
  (`self.RestartPlayer`))

(event `UpdateShipMesh`
  (params (NewShipMesh :type "StaticMesh Object Reference"))
  (bind _shipmesh (`self.ShipMesh`))
  ;[0.15 0.1031 0.006353 0.5] Update Ship Select Static Mesh
  (`StaticMeshComponent.SetStaticMesh` _shipmesh NewShipMesh)
  (`SceneComponent.K2_SetRelativeTransform` _shipmesh (`KismetMathLibrary.MakeTransform` (-2.599999 0.0 20.0) (struct :`Yaw` -90.0 :`Roll` 90.0) (20.0 22.2925 1.0)) false false))

(event `RestartPlayer`
  (bind _bp_killable (`self.BP_Killable`))
  ;[1 1 1] Ensure pawn stops moving
  (set `self.CanMove` false)
  (`KismetSystemLibrary.Delay` 0.05)
  ;[1 1 1] Reset to center of screen
  (`self.K2_SetActorLocationAndRotation` (0.0 0.0 0.0) (struct) false true)
  ;[1 1 1] Restore health
  (set `/Game/Blueprints/BP_Killable.CurrentHealth` (`/Game/Blueprints/BP_Killable.MaxHealth` _bp_killable) _bp_killable)
  ;[1 1 1] Restore movement after a short delay
  (`KismetSystemLibrary.Delay` 0.5)
  (set `self.CanMove` true))

(event `EnhancedInput|/Game/Input/IA_Shoot`
  (params (ActionValue :type Boolean) (ElapsedSeconds :type "Float (double-precision)") (TriggeredSeconds :type "Float (double-precision)") (InputAction :type "InputAction Object Reference" :default "/Game/Input/IA_Shoot.IA_Shoot"))
  (:`Started`
    ;[1 1 1] Turn shooting on/off
    (set `self.IsShooting` true))
  (:`Completed`
    (set `self.IsShooting` false)))

(event `ApplyShipData`
  (params (ShipData :type "/Game/Blueprints/BP_ShipData Object Reference"))
  (set `self.ShipData` ShipData)
  (`self.UpdateShipMesh` (`/Game/Blueprints/BP_ShipData.ShipMesh` ShipData))
  (set `self.FireRate` (`/Game/Blueprints/BP_ShipData.FireRate` (`self.ShipData`)))
  (set `self.CurrentLives` (`/Game/Blueprints/BP_ShipData.Lives` (`self.ShipData`))))

(event `EnhancedInput|/Game/Input/IA_Thrust`
  (params (ActionValue :type Boolean) (ElapsedSeconds :type "Float (double-precision)") (TriggeredSeconds :type "Float (double-precision)") (InputAction :type "InputAction Object Reference" :default "/Game/Input/IA_Thrust.IA_Thrust"))
  (:`Triggered`
    ;[1 1 1] Can the ship move?
    (if (`self.CanMove`)
      ;[1 1 1] Yes. Set acceleration.
      (set `FloatingPawnMovement.Acceleration` 8000.0 (`self.FloatingPawnMovement`))
      ;[1 1 1] Set the Direction vector.
      (set `self.Direction` (`self.GetActorForwardVector` self))))
  (:`Completed`
    ;[1 1 1] Stop accelerating
    (set `FloatingPawnMovement.Acceleration` 0.0 (`self.FloatingPawnMovement`))))

(event `EnhancedInput|/Game/Input/IA_Rotate`
  (params (ActionValue :type "Float (double-precision)") (ElapsedSeconds :type "Float (double-precision)") (TriggeredSeconds :type "Float (double-precision)") (InputAction :type "InputAction Object Reference" :default "/Game/Input/IA_Rotate.IA_Rotate"))
  (:`Triggered`
    ;[1 1 1] Can the ship move?
    (if (`self.CanMove`)
      ;[1 1 1] Yes. Rotate left/right
      (`SceneComponent.K2_AddWorldRotation` (`self.DefaultSceneRoot`) (`KismetMathLibrary.MakeRotator` 0.0 0.0 (* ActionValue (`self.TurnRate`) (`GameplayStatics.GetWorldDeltaSeconds`))) false false))))

(event `SetInvulnerable`
  (params (Condition :type Boolean))
  (if Condition
    (`PrimitiveComponent.SetSimulatePhysics` (`self.Sphere`) false)
    (`PrimitiveComponent.SetCollisionEnabled` (`self.Sphere`) "NoCollision")
    (else
      (`PrimitiveComponent.SetSimulatePhysics` (`self.Sphere`) false)
      (`PrimitiveComponent.SetCollisionEnabled` (`self.Sphere`) "QueryAndPhysics"))))

(event `Blink`
  (`/Engine/EditorBlueprintResources/StandardMacros.FlipFlop`
    (:`A`
      (`MeshComponent.SetVectorParameterValueOnMaterials` (`self.ShipMesh`) "Color" (1.0 1.0 1.0)))
    (:`B`
      (`MeshComponent.SetVectorParameterValueOnMaterials` (`self.ShipMesh`) "Color" (0.0 1.0 0.0)))))

(fn `InitializePlayer`
  (params (Lives :type Integer))
  (set `self.CurrentLives` Lives))

(fn `UserConstructionScript`
  (`parent.UserConstructionScript`))