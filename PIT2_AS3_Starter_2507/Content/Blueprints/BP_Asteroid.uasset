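; BP_Asteroid is an asteroid that comes in three sizes, damages the player on contact and can break apart when destroyed.
; Construction sets its color and scale by Type, and BeginPlay picks a random planar direction and a size-based speed, faster for smaller types.
; Overlap damages BP_Player unless invulnerable.
; HandleCollision notifies the spawner, destroys the actor, then asks the spawner to break it apart at the saved location.
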(event `self.ReceiveBeginPlay`
  (bind (_returnvalue_x _returnvalue_y) (`KismetMathLibrary.BreakVector` (* (`KismetMathLibrary.RandomUnitVector`) (`KismetMathLibrary.RandomFloatInRange` 0.0 360.0))))
  ;[1 1 1] I've Adjusted the speeds to be a lot slower than the defaults you may see in the document for easier testing -Murphy (Feel free to changes these values further while testing but make sure they are not so low during submission they appear not to be moving
  (`parent.ReceiveBeginPlay`)
  (set `FloatingPawnMovement.MaxSpeed` (select `/Game/Blueprints/E_AsteroidType` (`self.Type`) :`NewEnumerator0` (`KismetMathLibrary.RandomFloatInRange` 1000.0 1100.0) :`NewEnumerator1` (`KismetMathLibrary.RandomFloatInRange` 800.0 900.0) :`NewEnumerator2` (`KismetMathLibrary.RandomFloatInRange` 500.0 600.0)) (`self.FloatingPawnMovement`))
  (set `self.Direction` (`KismetMathLibrary.MakeVector` _returnvalue_x _returnvalue_y)))

(event `self.Sphere1.OnComponentBeginOverlap`
  (params (OverlappedComponent :type "PrimitiveComponent Object Reference") (OtherActor :type "Actor Object Reference") (OtherComp :type "PrimitiveComponent Object Reference") (OtherBodyIndex :type Integer) (bFromSweep :type Boolean) (SweepResult :type "HitResult Structure (by ref)"))
  (bind _asbp_player (cast `/Game/Blueprints/BP_Player` OtherActor))
  (if (not (`/Game/Blueprints/BP_Player.IsInvulnerable` _asbp_player))
    (`GameplayStatics.ApplyDamage` _asbp_player 1.0 null self)))

(event `self.HandleCollision`
  (bind _spawnerref (`self.SpawnerRef`))
  ;[1 0.8167 0.05079 0.3478] Remember Asteroid Location upon Death
  (set `self.DeathLocation` (`SceneComponent.K2_GetComponentLocation` (`self.DefaultSceneRoot`)))
  (`/Game/Blueprints/BP_Spawner.AsteroidDestroyed` _spawnerref (`self.Type`))
  ;[0.15 0.1295 0.008343 0.5] Destroy asteroid
  (`self.K2_DestroyActor`)
  ;[0.15 0.1249 0.00777 0.5] Tell Spawner to break apart this asteroid
  (`/Game/Blueprints/BP_Spawner.BreakApart` _spawnerref (`self.Type`) (`self.DeathLocation`)))

(fn `UserConstructionScript`
  (`parent.UserConstructionScript`)
  (`MeshComponent.SetVectorParameterValueOnMaterials` (`self.Sphere`) "Color" (`KismetMathLibrary.Conv_LinearColorToVector` (`self.Color`)))
  (`SceneComponent.SetWorldScale3D` (`self.Sphere`) (select `/Game/Blueprints/E_AsteroidType` (`self.Type`) :`NewEnumerator0` (`self.SmallSize`) :`NewEnumerator1` (`self.MediumSize`) :`NewEnumerator2` (`self.LargeSize`)))
  (`SphereComponent.SetSphereRadius` (`self.Sphere1`) 50.0 true))