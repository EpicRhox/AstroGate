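; Spawner actor for an Asteroids-style game that manages waves, asteroid splitting and score awards.
; Each wave spawns as many large asteroids as the wave number at random HUD-converted screen edges.
; BreakApart splits large and medium asteroids into smaller ones, adds points through BP_GameMode and advances the wave when none remain.
; It also rebuilds saved waves with velocities and clears all asteroids when the HUD's main-menu-clearing event fires.
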(event `self.ReceiveBeginPlay`
  ;[0.15 0.1196 0.01205 0.5] Wait for HUD to load
  (`KismetSystemLibrary.Delay` 0.1)
  ;[0.15 0.1202 0.0227 0.5] Get HUD reference
  (bind _asbp_hud (cast `/Game/Blueprints/BP_HUD` (`PlayerController.GetHUD` (`GameplayStatics.GetPlayerController` 0))))
  (set `self.HUD` _asbp_hud)
  (add `/Game/Blueprints/BP_HUD.ClearMainMenu` (`self.HUD`) (delegate `HandleClearingMainMenu`))
  (add `self.AsteroidSpawned` (delegate `OnEnemySpawned`)))

(event `OnEnemySpawned` :!signature `self.AsteroidSpawned`
  (params (Type :type "/Game/Blueprints/E_AsteroidType Enum" :default "NewEnumerator0"))
  (bind _activeasteroids (`self.ActiveAsteroids`))
  (`BlueprintMapLibrary.Map_Add` _activeasteroids Type (+ (`BlueprintMapLibrary.Map_Find` _activeasteroids Type) 1)))

(event `HandleClearingMainMenu`
  (`self.RestartGame`))

(event `SpawnAsteroid`
  (params (SpawnWorldLocation :type "Vector Structure") (Type :type "/Game/Blueprints/E_AsteroidType Enum" :default "NewEnumerator0"))
  ;[0.15 0.1436 0.01436 0.5] Spawn an asteroid of a given type at a given world location
  (`|SpawnActorFromClass` "/Game/Blueprints/BP_Asteroid.BP_Asteroid_C" (`KismetMathLibrary.MakeTransform` SpawnWorldLocation) "Undefined" "MultiplyWithRoot" null Type self null))

(event `SpawnWave`
  (`self.NewWaveSpawned`)
  ;[0.15 0.1367 0.006187 0.5] Do this <CurrentWave> times
  (for _ (range (`self.CurrentWave`))
    ;[0.15 0.1183 0.01102 0.5] Get a random screen edge and convert it to world coordinates
    (bind _worldposition (`/Game/Blueprints/BP_HUD.ConvertToWorldPosition` (`self.HUD`) (`KismetArrayLibrary.Array_Random` (`|MakeArray` "NewEnumerator0" "NewEnumerator1" "NewEnumerator2" "NewEnumerator3" :!type "/Game/Blueprints/E_SpawnLocation Enum"))))
    ;[0.15 0.1386 0.01207 0.5] Spawn Large Asteroid at coordinates
    (`self.SpawnAsteroid` _worldposition "NewEnumerator2")))

(event `BreakApart`
  (params (Type :type "/Game/Blueprints/E_AsteroidType Enum" :default "NewEnumerator0") (Location :type "Vector Structure"))
  (`|ExecutionSequence`
    (:`then_0`
      ;[0.15 0.1061 0.01245 0.5] Check asteroids type
      (switch `/Game/Blueprints/E_AsteroidType` Type
        (:`NewEnumerator1`
          ;[0.15 0.1239 0.01215 0.5] Medium.  Spawn 3 small asteroids
          (for _ (range 3)
            (`self.SpawnAsteroid` Location)))
        (:`NewEnumerator2`
          ;[0.15 0.1324 0.003163 0.5] Large. Spawn 2 medium asteroids
          (for _ (range 2)
            (`self.SpawnAsteroid` Location "NewEnumerator1")))))
    (:`then_1`
      ;[0.15 0.03329 0.001732 0.5] Upon breaking asteroid, add respective points to score
      (switch `/Game/Blueprints/E_AsteroidType` Type
        (:`NewEnumerator0`
          (`self.PointsAdd` (`self.SmallPoints`)))
        (:`NewEnumerator1`
          (`self.PointsAdd` (`self.MediumPoints`)))
        (:`NewEnumerator2`
          (`self.PointsAdd` (`self.LargePoints`)))))
    (:`then_2`
      ;[0.15 0.128 0.01592 0.5] Out of Asteroids?
      (bind _outactors (`GameplayStatics.GetAllActorsOfClass` "/Game/Blueprints/BP_Asteroid.BP_Asteroid_C"))
      (if (<= (`KismetArrayLibrary.Array_Length` _outactors) 0)
        ;[0.15 0.1218 0.008737 0.5] Yes. Spawn the next wave
        (`/Engine/EditorBlueprintResources/StandardMacros.IncrementInt` (`self.CurrentWave`)
          (:`  `
            (`self.SpawnWave`)))))))

(event `/Game/Blueprints/BPI_RestartGame.RestartGame`
  ;[0.15 0.1102 0.01095 0.5] Remove all asteroids from the map
  (bind _outactors (`GameplayStatics.GetAllActorsOfClass` "/Game/Blueprints/BP_Asteroid.BP_Asteroid_C"))
  (for _array_element _outactors
    (`self.K2_DestroyActor` _array_element)))

(event `/Game/Blueprints/BPI_SpawnerComms.AsteroidDestroyed`
  (params (AsteroidType :type "/Game/Blueprints/E_AsteroidType Enum" :default "NewEnumerator0")))

(event `LoadWaveFromSave`
  (params (EnemyToSpawn :type "Array of /Game/Blueprints/F_EnemySaveData Structure"))
  (for _array_element EnemyToSpawn
    (bind (_transform _velocity _type) (break `/Game/Blueprints/F_EnemySaveData` _array_element))
    (bind _returnvalue (`|SpawnActorFromClass` "/Game/Blueprints/BP_Asteroid.BP_Asteroid_C" _transform "Undefined" "MultiplyWithRoot" null _type self null))
    (set `MovementComponent.Velocity` _velocity (`/Game/Blueprints/BP_Movement.FloatingPawnMovement` _returnvalue))
    (`self.AsteroidSpawned` _type)))

(fn `PointsAdd`
  (params (Points :type Integer))
  (bind _asbp_game_mode (cast `/Game/Blueprints/BP_GameMode` (`GameplayStatics.GetGameMode`)))
  (`/Game/Blueprints/BP_GameMode.AddPoints` _asbp_game_mode Points))

(fn `UserConstructionScript`)