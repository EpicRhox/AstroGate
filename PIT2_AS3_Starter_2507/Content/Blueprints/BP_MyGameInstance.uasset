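; BP_MyGameInstance is the game instance that loads a saved game from a numbered slot.
; LoadGame builds the slot name from the index, checks that the save exists, and casts it to BP_GameSave.
; It copies saved score, wave, lives and spawned count into temporary variables, sets a loading flag, then opens Level1, so the state survives the level change.
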(fn `LoadGame`
  (params (SlotIndex :type Integer))
  (bind _returnvalue (`KismetStringLibrary.Concat_StrStr` "SaveSlot_" (`KismetStringLibrary.Conv_IntToString` SlotIndex)))
  (bind _returnvalue_2 (`GameplayStatics.DoesSaveGameExist` _returnvalue))
  (if _returnvalue_2
    (bind _returnvalue_3 (`GameplayStatics.LoadGameFromSlot` _returnvalue))
    (bind _asbp_game_save (cast `/Game/Blueprints/BP_GameSave` _returnvalue_3))
    (bind _output_get (set `self.GameSaveBP` _asbp_game_save))
    (set `self.TempSavedScore` (`/Game/Blueprints/BP_GameSave.SavedScore` _output_get))
    (set `self.TempSavedWave` (`/Game/Blueprints/BP_GameSave.SavedWave` (`self.GameSaveBP`)))
    (set `self.TempSavedLives` (`/Game/Blueprints/BP_GameSave.SavedLives` (`self.GameSaveBP`)))
    (set `self.TempSavedSpawned` (`/Game/Blueprints/BP_GameSave.SavedSpawned` (`self.GameSaveBP`)))
    (set `self.bIsLoadingFromSave` true)
    (`GameplayStatics.OpenLevel` "Level1")))